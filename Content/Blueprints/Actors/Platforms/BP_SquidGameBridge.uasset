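; Glass-bridge style actor, named after Squid Game, with two side-by-side platforms, one of which is fake.
; BeginPlay randomly picks the left or right platform as fake and applies the M_Door material to it.
; Player 0's character overlapping either side's trigger makes the fake platform simulate physics, then destroys it five seconds later.
; Both triggers share this logic, so the fake drops whichever side is entered.
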(event OnComponentBeginOverlap(LeftCol)
  (params (OverlappedComponent :type Primitive%20Component%20Object%20Reference) (OtherActor :type Actor%20Object%20Reference) (OtherComp :type Primitive%20Component%20Object%20Reference) (OtherBodyIndex :type Integer) (bFromSweep :type Boolean) (SweepResult :type Hit%20Result%20Structure%20%28by%20ref%29))
  (bind _fakeplatform (Variables|Default|GetFakePlatform))
  (Variables|Default|SetActorToCheck OtherActor)
  (if (== (Variables|Default|GetActorToCheck) (Game|GetPlayerCharacter 0))
    (Utilities|IsValid (Variables|Default|GetFakePlatform)
      (:Is%20Valid
        (Physics|SetSimulatePhysics _fakeplatform true)
        (Utilities|FlowControl|Delay 5.0)
        (Components|DestroyComponent _fakeplatform)))))

(event OnComponentBeginOverlap(RightCol)
  (params (OverlappedComponent :type Primitive%20Component%20Object%20Reference) (OtherActor :type Actor%20Object%20Reference) (OtherComp :type Primitive%20Component%20Object%20Reference) (OtherBodyIndex :type Integer) (bFromSweep :type Boolean) (SweepResult :type Hit%20Result%20Structure%20%28by%20ref%29))
  (bind _fakeplatform (Variables|Default|GetFakePlatform))
  (Variables|Default|SetActorToCheck OtherActor)
  (if (== (Variables|Default|GetActorToCheck) (Game|GetPlayerCharacter 0))
    (Utilities|IsValid (Variables|Default|GetFakePlatform)
      (:Is%20Valid
        (Physics|SetSimulatePhysics _fakeplatform true)
        (Utilities|FlowControl|Delay 5.0)
        (Components|DestroyComponent _fakeplatform)))))

(event EventBeginPlay
  (if (== (Math|Random|RandomIntegerinRange 0 1) 0)
    (Variables|Default|SetIsLeftFake? true)
    (Variables|Default|SetFakePlatform (Variables|Default|GetLeftPlatform))
    (else
      (Variables|Default|SetIsLeftFake? false)
      (Variables|Default|SetFakePlatform (Variables|Default|GetRigtPlatform))))
  (Rendering|Material|SetMaterial (Variables|Default|GetFakePlatform) 0 "/Game/StarterContent/Props/Materials/M_Door.M_Door"))

(fn ConstructionScript)
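; BP_Platform is a falling platform that drops after the player character touches it, then resets itself.
; On BeginPlay it caches the Platform component's world transform.
; A Box overlap by player 0's character waits briefly, enables physics simulation on Platform, then after a longer delay disables it and teleports Platform back to the cached transform.
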(event OnComponentBeginOverlap(Box)
  (params (OverlappedComponent :type Primitive%20Component%20Object%20Reference) (OtherActor :type Actor%20Object%20Reference) (OtherComp :type Primitive%20Component%20Object%20Reference) (OtherBodyIndex :type Integer) (bFromSweep :type Boolean) (SweepResult :type Hit%20Result%20Structure%20%28by%20ref%29))
  (bind _platform (Variables|Default|GetPlatform))
  (if (== OtherActor (Game|GetPlayerCharacter 0))
    (Utilities|FlowControl|Delay 1.0)
    (Physics|SetSimulatePhysics _platform true)
    (Utilities|FlowControl|Delay 5.0)
    (Physics|SetSimulatePhysics _platform false)
    (Transformation|SetWorldTransform _platform (Variables|Default|GetDefaultTransform) false true)))

(event EventBeginPlay
  (Variables|Default|SetDefaultTransform (Transformation|GetWorldTransform (Variables|Default|GetPlatform))))

(fn ConstructionScript)